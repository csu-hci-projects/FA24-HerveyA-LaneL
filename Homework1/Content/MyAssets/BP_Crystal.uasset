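; BP_Crystal is a destructible crystal actor with a health bar widget that loses health when damaged.
; On BeginPlay it passes current and max health to its WB_HealthForEnemy widget.
; When the first-person character overlaps its sphere, it damages itself and plays an explosion sound.
; AnyDamage scales incoming damage by 100, updates the bar, and at zero health spawns an attached emitter and destroys the actor.
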(event OnComponentBeginOverlap(Sphere)
  (params (OverlappedComponent :type Primitive%20Component%20Object%20Reference) (OtherActor :type Actor%20Object%20Reference) (OtherComp :type Primitive%20Component%20Object%20Reference) (OtherBodyIndex :type Integer) (bFromSweep :type Boolean) (SweepResult :type Hit%20Result%20Structure%20%28by%20ref%29))
  ;[1 1 1] Apply Damage
  (Utilities|Casting|CastToBP_FirstPersonCharacter OtherActor)
  (Game|Damage|ApplyDamage self 0.5 0 0)
  (Audio|PlaySound2D "/Game/StarterContent/Audio/Explosion_Cue.Explosion_Cue" 1.0 1.0 0.0 0 0))

(event EventBeginPlay
  ;[1 1 1] Set Current Health
  (bind _aswb_health_for_enemy (Utilities|Casting|CastToWB_HealthForEnemy (UserInterface|GetUserWidgetObject (Variables|Default|GetWidget))))
  (bind _output_get (Variables|Default|SetWB%20Health%20For%20Enemy _aswb_health_for_enemy))
  (Variables|/Game/UI/WB_HealthForEnemy.WB_HealthForEnemy_C|SetCurrentHealth _output_get (Variables|Default|GetCurrentHealth))
  (Variables|/Game/UI/WB_HealthForEnemy.WB_HealthForEnemy_C|SetMaxHealth _output_get (Variables|Default|GetMaxHealth)))

(event Game|Damage|EventAnyDamage
  (params (Damage :type Float%20%28single-precision%29) (DamageType :type Damage%20Type%20Object%20Reference) (InstigatedBy :type Controller%20Object%20Reference) (DamageCauser :type Actor%20Object%20Reference))
  (bind _output_get (Variables|Default|SetCurrentHealth (- (Variables|Default|GetCurrentHealth) (* Damage 1e+02))))
  (Default|UpdateHealth (Variables|Default|GetWB%20Health%20For%20Enemy) (Math|Integer|Clamp(Integer) _output_get 0 (Variables|Default|GetMaxHealth)))
  (if (<= (Variables|Default|GetCurrentHealth) 0)
    (Effects|SpawnEmitterAttached 0 (Variables|Default|GetCrystal) "None")
    (Actor|DestroyActor)))

(fn ConstructionScript)