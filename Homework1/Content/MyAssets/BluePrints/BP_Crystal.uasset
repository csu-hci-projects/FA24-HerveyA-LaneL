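; BP_Crystal is a destructible target crystal with a health bar that counts toward ending the game.
; On BeginPlay it seeds its WB_HealthForEnemy widget with current and max health.
; Hits from BP_FirstPersonProjectile make it damage itself, and AnyDamage scales that damage, lowers health and updates the widget.
; At zero health it spawns an emitter, destroys itself, decrements the player's TargetHit count and calls EndGame when that reaches zero.
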(event Collision|EventHit
  (params (MyComp :type Primitive%20Component%20Object%20Reference) (Other :type Actor%20Object%20Reference) (OtherComp :type Primitive%20Component%20Object%20Reference) (bSelfMoved :type Boolean) (HitLocation :type Vector :default "0, 0, 0") (HitNormal :type Vector :default "0, 0, 0") (NormalImpulse :type Vector :default "0, 0, 0") (Hit :type Hit%20Result%20Structure%20%28by%20ref%29))
  ;[1 1 1] Apply Damage
  (Utilities|Casting|CastToBP_FirstPersonProjectile Other)
  (Game|Damage|ApplyDamage self 0.5 0 0))

(event EventBeginPlay
  ;[1 1 1] Set Current Health
  (bind _aswb_health_for_enemy (Utilities|Casting|CastToWB_HealthForEnemy (UserInterface|GetUserWidgetObject (Variables|Default|GetWidget))))
  (bind _output_get (Variables|Default|SetWB%20Health%20For%20Enemy _aswb_health_for_enemy))
  (Variables|/Game/UI/WB_HealthForEnemy.WB_HealthForEnemy_C|SetCurrentHealth _output_get (Variables|Default|GetCurrentHealth))
  (Variables|/Game/UI/WB_HealthForEnemy.WB_HealthForEnemy_C|SetMaxHealth _output_get (Variables|Default|GetMaxHealth)))

(event Game|Damage|EventAnyDamage
  (params (Damage :type Float%20%28single-precision%29) (DamageType :type Damage%20Type%20Object%20Reference) (InstigatedBy :type Controller%20Object%20Reference) (DamageCauser :type Actor%20Object%20Reference))
  (bind _output_get (Variables|Default|SetCurrentHealth (- (Variables|Default|GetCurrentHealth) (* Damage 1e+02))))
  (Default|UpdateHealth (Variables|Default|GetWB%20Health%20For%20Enemy) (Math|Integer|Clamp(Integer) _output_get 0 (Variables|Default|GetMaxHealth)))
  (if (<= (Variables|Default|GetCurrentHealth) 0)
    (Effects|SpawnEmitterAttached 0 (Variables|Default|GetCrystal) "None")
    (Actor|DestroyActor)
    (bind _asbp_first_person_character (Utilities|Casting|CastToBP_FirstPersonCharacter (Game|GetPlayerCharacter 0)))
    (bind _result (Math|Integer|DecrementInt (Variables|/Game/FirstPerson/Blueprints/BP_FirstPersonCharacter.BP_FirstPersonCharacter_C|GetTarget%20Hit _asbp_first_person_character))
      (:%20%20
        (if (== _result 0)
          (Default|EndGame _asbp_first_person_character))))))

(fn ConstructionScript)